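; BP_SpeedCamChanger is a trigger that changes the camera's spline speed (VitesseSurLaSpline on BP_Cam) when BP_Tic enters its box.
; On overlap it moves an Arrow to the player and compares its relative X with a Witness component to detect crossing direction.
; One direction saves the current speed and plays a timeline blending to NewSpeedCam; the other reverses it back to the saved speed.
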(event OnComponentBeginOverlap(Box)
  (params (OverlappedComponent :type Primitive%20Component%20Object%20Reference) (OtherActor :type Actor%20Object%20Reference) (OtherComp :type Primitive%20Component%20Object%20Reference) (OtherBodyIndex :type Integer) (bFromSweep :type Boolean) (SweepResult :type Hit%20Result%20Structure%20%28by%20ref%29))
  (bind _asbp_tic (Utilities|Casting|CastToBP_Tic OtherActor)
    (:then
      (Transformation|SetWorldLocationAndRotation (Variables|Default|GetArrow) (Transformation|GetWorldLocation (Variables|/Script/Engine.Character|GetCapsuleComponent _asbp_tic)) (Transformation|GetWorldRotation (Variables|/Script/Engine.Character|GetCapsuleComponent _asbp_tic)) false false)
      (Variables|Default|SetVitesseSplineReference (Variables|/Game/Blueprints/Camera/CameraRails/BP_Cam.BP_Cam_C|GetVitesse%20sur%20la%20Spline (Variables|Default|GetCameraReference)))
      (CallFunction|ChecktheWay))
    (:CastFailed
      (Development|PrintString "Cast Player Failed" true true "(R=1.000000,G=0.000000,B=0.000000,A=1.000000)"))))

(event Custom|CheckTheWay
  (if (< (.x (Variables|/Script/Engine.SceneComponent|GetRelativeLocation (Variables|Default|GetArrow))) (.x (Variables|/Script/Engine.SceneComponent|GetRelativeLocation (Variables|Default|GetWitness))))
    (Variables|Default|SetVitesseSlineAncienneReference (Variables|Default|GetVitesseSplineReference))
    (bind _newspeedvalue (Timeline|Transitioning_Speed Play)
      (:Update
        (Variables|/Game/Blueprints/Camera/CameraRails/BP_Cam.BP_Cam_C|SetVitesse%20sur%20la%20Spline (Variables|Default|GetCameraReference) (Math|Float|Lerp (Variables|Default|GetVitesseSlineAncienneReference) (Variables|Default|GetNewSpeedCam) _newspeedvalue)))
      (:Finished
        (Development|PrintString (Utilities|String|ToString(Float) (Variables|Default|GetVitesseSplineReference)))
        (Development|PrintString (Utilities|String|ToString(Float) (Variables|Default|GetVitesseSlineAncienneReference)))))
    (else
      (Timeline|Transitioning_Speed Reverse))))

(event EventBeginPlay
  (bind _returnvalue (Actor|GetActorOfClass "/Game/Blueprints/Camera/CameraRails/BP_Cam.BP_Cam_C"))
  (bind _output_get (Variables|Default|SetCameraReference _returnvalue))
  (bind _output_get_2 (Variables|Default|SetVitesseSplineReference (Variables|/Game/Blueprints/Camera/CameraRails/BP_Cam.BP_Cam_C|GetVitesse%20sur%20la%20Spline _output_get)))
  (Development|PrintString (Utilities|String|ToString(Float) _output_get_2)))

(fn ConstructionScript)