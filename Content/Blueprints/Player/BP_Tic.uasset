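; Tic player character Blueprint that follows the player-one split-screen camera and handles light combo and charged melee-style attacks.
; Light attacks chain numbered sections of one montage, using Buffer notify windows to queue the next hit and End Combo to stop.
; Holding charged attack plays a montage and Niagara effect while accumulating charge.
; Release jumps to the Attack section at full charge, otherwise cancels the montage.
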(event Custom|Combo
  (params (IndexCombo :type Integer))
  ;[1 1 1] Attack
  ;;[0.1248 0.4423 1] SimpleCombo
  (bind _notifyname (Animation|Montage|PlayMontage (Variables|Character|GetMesh) "/Game/Animation/Player/AnimMontage/AM_Combo01.AM_Combo01" 1.8 0.0 (Utilities|String|StringToName (Utilities|String|Append "Attack0" (Utilities|String|ToString(Integer) IndexCombo))))
    (:OnCompleted
      (Variables|Default|Setb_IsInCombo false))
    (:OnNotifyBegin
      (switch name _notifyname
        (:Buffer
          (Variables|Default|Setb_WantCombo false))
        (:EndCombo
          (Animation|StopAnimMontage "/Game/Animation/Player/AnimMontage/AM_Combo01.AM_Combo01")
          (Variables|Default|Setb_WantCombo false)
          (Variables|Default|Setb_IsInCombo false))))
    (:OnNotifyEnd
      (if (== _notifyname "Buffer")
        (if (Variables|Default|Getb_WantCombo)
          (CallFunction|Combo (+ IndexCombo 1)))))))

(event Custom|Charged
  ;[1 1 1] Attack
  ;;[0.2077 0.627 1] ChargedAttack
  ;;;[0.4283 1 0.4172] Charged the attack
  (if (not (and (Variables|Default|Getb_IsInCombo) (Variables|Default|GetIsInCharged)))
    (Animation|Montage|PlayMontage (Variables|Character|GetMesh) "/Game/Animation/Player/ChargedAttack/NewAnimMontage.NewAnimMontage" 1.0 0.0 (Utilities|Name|MakeLiteralName "Default")
      (:then
        (Variables|Default|SetIsInCharged true))
      (:OnInterrupted
        (Variables|Default|SetIsInCharged false)
        (Variables|Default|Setb_IsInCombo false)))))

(event Custom|Release
  ;[1 1 1] Attack
  ;;[0.2077 0.627 1] ChargedAttack
  ;;;[1 0.2865 0.2865] Release the attack
  (if (not (>= (Variables|Default|GetChargedTime) (Variables|Default|GetMaxChargedTime)))
    (Animation|StopAnimMontage "/Game/Animation/Player/ChargedAttack/NewAnimMontage.NewAnimMontage")
    (Variables|Default|SetChargedTime 0.0)
    (elif (not (Variables|Default|GetCanBlend))
      (Animation|Montage|PlayMontage (Variables|Character|GetMesh) "/Game/Animation/Player/ChargedAttack/NewAnimMontage.NewAnimMontage" 1.0 0.0 (Utilities|Name|MakeLiteralName "Attack")
        (:then
          (Variables|Default|SetCanBlend true)
          (Variables|Default|SetIsInCharged true)
          (Variables|Default|SetChargedTime 0.0))
        (:OnCompleted
          (Variables|Default|SetIsInCharged false)
          (Variables|Default|SetCanBlend false :!label _label))
        (:OnInterrupted
          (goto _label))))))

(event Input|EnhancedActionEvents|EnhancedInputActionIA_Attack
  (params (ActionValue :type Boolean) (ElapsedSeconds :type Float%20%28double-precision%29) (TriggeredSeconds :type Float%20%28double-precision%29) (InputAction :type Input%20Action%20Object%20Reference :default "/Game/Input/Actions/IA_Attack.IA_Attack"))
  ;[1 1 1] Attack Input
  (:Started
    (if (not (Variables|Default|GetIsInCharged))
      (if (Variables|Default|Getb_IsInCombo)
        (Variables|Default|Setb_WantCombo true)
        (else
          (Variables|Default|Setb_IsInCombo true)
          (CallFunction|Combo 1))))))

(event Input|EnhancedActionEvents|EnhancedInputActionIA_ChargedAttack
  (params (ActionValue :type Boolean) (ElapsedSeconds :type Float%20%28double-precision%29) (TriggeredSeconds :type Float%20%28double-precision%29) (InputAction :type Input%20Action%20Object%20Reference :default "/Game/Input/Actions/IA_ChargedAttack.IA_ChargedAttack"))
  (bind _niagara (Variables|Default|GetNiagara))
  ;[1 1 1] Attack Input
  (:Triggered
    (Variables|Default|SetChargedTime (+ (Variables|Default|GetChargedTime) 0.1)))
  (:Started
    (CallFunction|Charged)
    (Components|Activation|Activate _niagara false))
  (:Completed
    (CallFunction|Release)
    (Components|Activation|Deactivate _niagara)))

(event EventTick
  (params (DeltaSeconds :type Float%20%28single-precision%29))
  ;[1 1 1] Update
  (bind _cameraref (Variables|Default|GetCameraRef)
    (:then
      (CallFunction|FollowCameraSplitScreen (Variables|/Game/Blueprints/Camera/CameraSplitScreen/Bp_CameraSplitP1.Bp_CameraSplitP1_C|GetCamera _cameraref)))
    (:else)))

(event EventBeginPlay
  ;[1 1 1] BeginPlay
  (|CallParentFunction)
  (bind _returnvalue (Actor|GetActorOfClass "/Game/Blueprints/Camera/CameraSplitScreen/Bp_CameraSplitP1.Bp_CameraSplitP1_C"))
  (Variables|Default|SetCameraRef _returnvalue))

(fn ConstructionScript)