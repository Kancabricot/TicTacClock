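; Playable character Tic, with a chained melee combo and player-one split-screen camera support.
; The action input starts the combo montage or queues the next hit while one is playing.
; Combo recurses through numbered montage sections: a Buffer notify window clears then checks the queued input, and End Combo stops the chain.
; BeginPlay caches the P1 split camera actor, which Tick passes to FollowCameraSplitScreen.
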(event Custom|Combo
  (params (IndexCombo :type Integer))
  (bind _notifyname (Animation|Montage|PlayMontage (Variables|Character|GetMesh) "/Game/Animation/Tac/Fight/AM_Combo01.AM_Combo01" 1.8 0.0 (Utilities|String|StringToName (Utilities|String|Append "Attack0" (Utilities|String|ToString(Integer) IndexCombo))))
    (:OnCompleted
      (Variables|Default|Setb_IsInCombo false))
    (:OnNotifyBegin
      (switch name _notifyname
        (:Buffer
          (Variables|Default|Setb_WantCombo false))
        (:EndCombo
          (Animation|StopAnimMontage "/Game/Animation/Tac/Fight/AM_Combo01.AM_Combo01")
          (Variables|Default|Setb_WantCombo false)
          (Variables|Default|Setb_IsInCombo false))))
    (:OnNotifyEnd
      (if (== _notifyname "Buffer")
        (if (Variables|Default|Getb_WantCombo)
          (CallFunction|Combo (+ IndexCombo 1)))))))

(event Input|EnhancedActionEvents|EnhancedInputActionIA_Action
  (params (ActionValue :type Boolean) (ElapsedSeconds :type Float%20%28double-precision%29) (TriggeredSeconds :type Float%20%28double-precision%29) (InputAction :type Input%20Action%20Object%20Reference :default "/Game/Input/Actions/IA_Action.IA_Action"))
  (:Started
    (if (Variables|Default|Getb_IsInCombo)
      (Variables|Default|Setb_WantCombo true)
      (else
        (Variables|Default|Setb_IsInCombo true)
        (CallFunction|Combo 1)))))

(event EventTick
  (params (DeltaSeconds :type Float%20%28single-precision%29))
  (bind _cameraref (Variables|Default|GetCameraRef)
    (:then
      (CallFunction|FollowCameraSplitScreen (Variables|/Game/Blueprints/CameraSplitScreen/Bp_CameraSplitP1.Bp_CameraSplitP1_C|GetCamera _cameraref)))
    (:else)))

(event EventBeginPlay
  (|CallParentFunction)
  (bind _returnvalue (Actor|GetActorOfClass "/Game/Blueprints/CameraSplitScreen/Bp_CameraSplitP1.Bp_CameraSplitP1_C"))
  (Variables|Default|SetCameraRef _returnvalue))

(fn ConstructionScript)