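; BP_Dummy is a dummy enemy with a health pool shown on a WG_LifeBar widget.
; SetLife subtracts damage and updates the bar, or destroys the actor once health would reach zero.
; Pressing P deals test damage and restarts the DelayHeal timeline, used as a timer.
; When that timeline finishes, health resets to maximum and a zero-damage SetLife call refreshes the bar.
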(event EventBeginPlay
  (bind _aswg_life_bar (Utilities|Casting|CastToWG_LifeBar (UserInterface|GetWidget (Variables|Default|GetWGUI))))
  (Variables|Refs|SetWGLifeBarRef _aswg_life_bar)
  (Variables|Default|SetActualHealth (Variables|Default|GetMaxHealth)))

(event Input|KeyboardEvents|P
  (params (Key :type Key%20Structure :default "None"))
  (:Pressed
    (CallFunction|SetLife 1e+01)
    (Utilities|FlowControl|Sequence
      (:then_0
        (Development|PrintString "TakeDamage"))
      (:then_1
        (Timeline|DelayHeal PlayFromStart
          (:Finished
            (Variables|Default|SetActualHealth (Variables|Default|GetMaxHealth))
            (Development|PrintString "SetMaxHealth")
            (CallFunction|SetLife 0.0)))))))

(fn ConstructionScript)

(fn SetLife
  (params (Damage :type Float%20%28double-precision%29))
  (if (<= (- (Variables|Default|GetActualHealth) Damage) 0.0)
    (Actor|DestroyActor)
    (else
      (bind _output_get (Variables|Default|SetActualHealth (- (Variables|Default|GetActualHealth) Damage)))
      (Default|SetLifeBar (Variables|Refs|GetWGLifeBarRef) _output_get (Variables|Default|GetMaxHealth)))))