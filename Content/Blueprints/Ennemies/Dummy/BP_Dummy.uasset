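; Training dummy enemy that takes hits from BP_Tic, shows health on a WG_LifeBar widget and can refill itself.
; Damage spawns FX at the attacker's mesh and calls SetLife, which plays camera shake, red material flash and hit animation, then lowers health.
; A lethal hit hides the dummy and disables collision without updating stored health.
; When stored health is 10 or less, a delayed timeline restores health, visibility and collision.
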(event Custom|RefillHealth
  (bind _dummy (Variables|Default|GetDummy))
  (bind _maxhealth (Variables|Default|GetMaxHealth))
  (bind _delay (Timeline|DelayHeal PlayFromStart)
    (:Update
      (Variables|Default|SetActualHealth _maxhealth)
      (Default|SetLifeBar (Variables|Refs|GetWGLifeBarRef) (Math|Float|Lerp (Variables|Default|GetActualHealth) _maxhealth _delay) _maxhealth)
      (Rendering|SetVisibility _dummy true false)
      (Collision|SetCollisionEnabled _dummy "QueryAndProbe"))))

(event Custom|DamageAnime
  (Class|LegacyCameraShake|StartLegacyCameraShake (Game|GetPlayerCameraManager 0) "/Game/Blueprints/Camera/CameraShake/BP_CamShakeHitAi.BP_CamShakeHitAi_C" 1.0 "CameraLocal" "0, 0, 0")
  (Rendering|Material|SetMaterial (Variables|Default|GetDummy) 0 "/Game/Art/Mesh/Materials/SimpleColors/M_Red.M_Red")
  (Utilities|FlowControl|Delay 0.1)
  (Rendering|Material|SetMaterial (Variables|Default|GetDummy) 0 "/Game/Art/Characters/Mannequin_UE4/Materials/M_MannequinUE4_Body.M_MannequinUE4_Body"))

(event EventDamage
  (params (DamageDo :type Float%20%28double-precision%29) (WhosIt :type Actor%20Object%20Reference))
  (bind _asbp_tic (Utilities|Casting|CastToBP_Tic WhosIt))
  (Niagara|SpawnSystematLocation "/Game/Art/Fx/HitImpact/FX.FX" (Transformation|GetWorldLocation (Variables|/Game/Blueprints/Player/BP_Tic.BP_Tic_C|GetStaticMesh1 _asbp_tic)))
  (Development|PrintString (Utilities|String|Append "Take damage : " (Utilities|String|ToString(Float) DamageDo)))
  (CallFunction|SetLife DamageDo (Transformation|GetWorldLocation (Variables|/Game/Blueprints/Player/BP_Tic.BP_Tic_C|GetStaticMesh1 _asbp_tic)))
  (if (<= (Variables|Default|GetActualHealth) 1e+01)
    (Utilities|FlowControl|Delay 2.0)
    (CallFunction|RefillHealth)))

(event EventBeginPlay
  (bind _aswg_life_bar (Utilities|Casting|CastToWG_LifeBar (UserInterface|GetWidget (Variables|Default|GetWGUI))))
  (Variables|Refs|SetWGLifeBarRef _aswg_life_bar)
  (Variables|Default|SetActualHealth (Variables|Default|GetMaxHealth)))

(fn ConstructionScript)

(fn SetLife
  (params (Damage :type Float%20%28double-precision%29) (Vec :type Vector))
  (bind _dummy (Variables|Default|GetDummy))
  (CallFunction|DamageAnime)
  (Components|Animation|PlayAnimation (Variables|Default|GetDummy) "/Game/Animation/Ennemies/Boss_ReactionHits_unedited.Boss_ReactionHits_unedited" false)
  (Development|PrintString "Hello")
  (if (<= (- (Variables|Default|GetActualHealth) Damage) 0.0)
    (Rendering|SetVisibility _dummy false false)
    (Collision|SetCollisionEnabled _dummy "NoCollision")
    (else
      (bind _output_get (Variables|Default|SetActualHealth (- (Variables|Default|GetActualHealth) Damage)))
      (Default|SetLifeBar (Variables|Refs|GetWGLifeBarRef) _output_get (Variables|Default|GetMaxHealth)))))