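; BP_Cam is a two-player camera that slides along a spline while looking at the players' midpoint.
; BeginPlay spawns a BP_CamTarget and gathers BP_Tic and BP_Tac.
; Each Tick centers the target between them, maps its distance from StartPointTarget, inverted against the start-to-finish length, onto the spline, then aims the camera at it.
; An unused Block event would throttle Tic's movement when the players separate too far.
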(event Custom|GoToSplineTimeline
  (bind _firstdistance (Variables|Default|GetFirstDistance))
  (bind _targetcamref (Variables|Default|GettargetCamRef))
  (bind _returnvalue (Class|GameplayStatics|GetActorArrayAverageLocation (Variables|Default|GetPlayerTab)))
  (Transformation|SetActorLocation _targetcamref _returnvalue false false)
  (Transformation|SetRelativeLocation (Variables|Default|GetCamera) (.location (Spline|GetTransformatDistanceAlongSpline (Variables|Default|GetSpline) (Math|Float|Lerp 0.0 (Spline|GetSplineLength (Variables|Default|GetSpline)) (Math|Float|NormalizetoRange (+ (* (Transformation|GetDistanceTo _targetcamref (Variables|Default|GetStartPointTarget)) -1.0) _firstdistance) 0.0 _firstdistance)) "Local" false)) false false)
  (Transformation|SetWorldRotation (Variables|Default|GetCamera) (Math|Rotator|FindLookatRotation (Transformation|GetWorldLocation (Variables|Default|GetCamera)) (Transformation|GetWorldLocation (Variables|/Script/Engine.Actor|GetRootComponent (Variables|Default|GettargetCamRef)))) false false))

(event Custom|Block
  (bind _player1ref (Variables|Default|GetPlayer1ref))
  (bind _player1ref_2 (Variables|Default|GetPlayer1ref))
  (bind _player2ref (Variables|Default|GetPlayer2Ref))
  (bind _charactermovement (Variables|/Script/Engine.Character|GetCharacterMovement _player1ref))
  (Utilities|IsValid _player1ref_2
    (:Is%20Valid
      (Utilities|IsValid _player2ref
        (:Is%20Valid
          (if (not (>= 1e+03 (Transformation|GetDistanceTo _player1ref_2 _player2ref)))
            (Variables|Default|Setdistance%20ancienne (Transformation|GetDistanceTo (Variables|Default|GetPlayer1ref) (Variables|Default|GetPlayer2Ref)))
            (Utilities|FlowControl|Delay 0.2)
            (if (not (>= (Transformation|GetDistanceTo (Variables|Default|GetPlayer1ref) (Variables|Default|GetPlayer2Ref)) (Variables|Default|Getdistance%20ancienne)))
              (Variables|/Script/Engine.CharacterMovementComponent|SetMaxWalkSpeed _charactermovement 5e+02)
              (Variables|/Script/Engine.CharacterMovementComponent|SetMaxAcceleration _charactermovement 5e+02)
              (Development|PrintString "500" true true "(R=0.000000,G=0.660000,B=1.000000,A=1.000000)" 0.001)
              (else
                (Variables|/Script/Engine.CharacterMovementComponent|SetMaxWalkSpeed (Variables|/Script/Engine.Character|GetCharacterMovement (Variables|Default|GetPlayer1ref)) 0.0)
                (Development|PrintString "0" true true "(R=0.000000,G=0.660000,B=1.000000,A=1.000000)" 0.01)))))))))

(event EventBeginPlay
  (bind _returnvalue (Game|SpawnActorfromClass "/Game/Blueprints/BP_CamTarget.BP_CamTarget_C" (Math|Transform|MakeTransform "0, 0, 0" "0, 0, 0" "1.000000,1.000000,1.000000") "Undefined" "MultiplyWithRoot" 0 0))
  (Variables|Default|SettargetCamRef _returnvalue)
  (Variables|Default|SetFirstDistance (Transformation|GetDistanceTo (Variables|Default|GetFinishPoint) (Variables|Default|GetStartPointTarget)))
  (Utilities|FlowControl|Delay 0.2)
  (bind _returnvalue_2 (Actor|GetActorOfClass "/Game/Blueprints/BP_Tic.BP_Tic_C"))
  (bind _output_get (Variables|Default|SetPlayer1ref _returnvalue_2))
  (Utilities|Array|Add (Variables|Default|GetPlayerTab) _output_get)
  (bind _returnvalue_3 (Actor|GetActorOfClass "/Game/Blueprints/BP_Tac.BP_Tac_C"))
  (bind _output_get_2 (Variables|Default|SetPlayer2Ref _returnvalue_3))
  (Utilities|Array|Add (Variables|Default|GetPlayerTab) _output_get_2))

(event EventTick
  (params (DeltaSeconds :type Float%20%28single-precision%29))
  (CallFunction|GotoSplineTimeline))

(fn ConstructionScript)