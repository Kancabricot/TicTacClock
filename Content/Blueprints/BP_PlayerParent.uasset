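; BP_PlayerParent is a player base Blueprint that adds an Enhanced Input mapping context for its player index and provides attack, mesh-visibility and special-form functions.
; The special input always selects Mecha and spawns BP_MechaMerge; ResetSpecial clears the state.
; Attack sphere-traces pawns ahead, sending damage only after the hit loop ends.
; Move input calls MovementForSpecial, whose forwarding to the Mecha is disconnected.
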(event Input|EnhancedActionEvents|EnhancedInputActionIA_Special
  (params (ActionValue :type Boolean) (ElapsedSeconds :type Float%20%28double-precision%29) (TriggeredSeconds :type Float%20%28double-precision%29) (InputAction :type Input%20Action%20Object%20Reference :default "/Game/Input/Actions/IA_Special.IA_Special"))
  (:Started
    (if (not (Variables|Default|Getb_IsInSpecial))
      (switch int (Math|Random|RandomInteger 0)
        (:0
          (bind _output_get (Variables|Default|SetEnumSpecial "NewEnumerator1"))
          (CallFunction|SetSpecial _output_get))))))

(event Input|EnhancedActionEvents|EnhancedInputActionIA_Move
  (params (ActionValue :type Vector%202D%20Structure) (ElapsedSeconds :type Float%20%28double-precision%29) (TriggeredSeconds :type Float%20%28double-precision%29) (InputAction :type Input%20Action%20Object%20Reference :default "/Game/Input/Actions/IA_Move.IA_Move"))
  (:Triggered
    (CallFunction|MovementforSpecial (.x ActionValue) (.y ActionValue))))

(event EventBeginPlay
  (bind _indexplayer (Variables|References|GetIndexPlayer))
  (bind _returnvalue (Game|GetPlayerController _indexplayer))
  (bind _returnvalue_2 (PlayerController|LocalPlayerSubsystems|GetEnhancedInputLocalPlayerSubsystem _returnvalue))
  (Development|PrintString (Utilities|String|ToString(Integer) _indexplayer))
  (Utilities|IsValid _returnvalue_2
    (:Is%20Valid
      (Input|AddMappingContext _returnvalue_2 (Variables|References|GetMappingContext) 0 "(bIgnoreAllPressedKeysUntilRelease=True,bForceImmediately=False)"))))

(fn ConstructionScript)

(fn Attack
  (params (Damage :type Float%20%28double-precision%29))
  (bind _returnvalue (Transformation|GetActorLocation))
  (bind _returnvalue_2 (Transformation|GetActorForwardVector))
  (bind _returnvalue_3 (* _returnvalue_2 1.5e+02))
  (bind _returnvalue_4 (+ _returnvalue _returnvalue_3))
  (Development|PrintString "Attack")
  (bind _outhits (Collision|MultiSphereTraceForObjects _returnvalue_4 _returnvalue_4 2e+02 (Utilities|Array|MakeArray "ObjectTypeQuery3") false 0 "None" true "(R=1.000000,G=0.000000,B=0.000000,A=1.000000)" "(R=0.000000,G=1.000000,B=0.000000,A=1.000000)" 0.5))
  (for _array_element _outhits
    _)
  (Class|BPIAllyHit|Damage(Message) (.HitActor (Collision|BreakHitResult _array_element)) Damage))

(fn SetVisible/Invisible
  (params (SetVisible :type Boolean))
  (Rendering|SetVisibility (Variables|Character|GetMesh) SetVisible true))

(fn MovementforSpecial
  (params (X :type Float%20%28double-precision%29) (Y :type Float%20%28double-precision%29)))

(fn SetSpecial
  (params (EnumSpecial :type Enum_Special%20Enum :default "NewEnumerator0"))
  (switch Utilities|FlowControl|Switch|SwitchonEnum_Special EnumSpecial
    (:NewEnumerator1
      (bind _returnvalue (Game|SpawnActorfromClass "/Game/Blueprints/Special/BP_MechaMerge.BP_MechaMerge_C" (Transformation|GetActorTransform) "Undefined" "MultiplyWithRoot" 0 0))
      (Variables|Special|SetMechaRef _returnvalue))))

(fn ResetSpecial
  (Variables|Default|SetEnumSpecial "NewEnumerator0")
  (Variables|Default|Setb_IsInSpecial false))