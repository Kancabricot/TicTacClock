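; Menu pawn that lets a player, identified by a player index, navigate and confirm in a player selection widget.
; BeginPlay adds an Enhanced Input mapping context to the local player subsystem of that index's controller.
; Move input past a horizontal threshold triggers the widget's left or right animation for that index, and Jump validates the player.
; Debug prints show the index on start and movement.
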(event Input|EnhancedActionEvents|EnhancedInputActionIA_Move
  (params (ActionValue :type Vector%202D%20Structure) (ElapsedSeconds :type Float%20%28double-precision%29) (TriggeredSeconds :type Float%20%28double-precision%29) (InputAction :type Input%20Action%20Object%20Reference :default "/Game/Input/Actions/IA_Move.IA_Move"))
  (:Triggered
    (Development|PrintString (Utilities|String|ToString(Integer) (Variables|Default|GetIndexPlayer)))
    (if (> (.x ActionValue) 4e+01)
      (Default|StartAnimRight (Variables|Refs|GetWGPlayerSelectionRef) (Variables|Default|GetIndexPlayer))
      (elif (< (.x ActionValue) -4e+01)
        (Default|StartAnimLeft (Variables|Refs|GetWGPlayerSelectionRef) (Variables|Default|GetIndexPlayer))))))

(event Input|EnhancedActionEvents|EnhancedInputActionIA_Jump
  (params (ActionValue :type Boolean) (ElapsedSeconds :type Float%20%28double-precision%29) (TriggeredSeconds :type Float%20%28double-precision%29) (InputAction :type Input%20Action%20Object%20Reference :default "/Game/Input/Actions/IA_Jump.IA_Jump"))
  (:Started
    (Default|ValidPlayer (Variables|Refs|GetWGPlayerSelectionRef) (Variables|Default|GetIndexPlayer))))

(event EventBeginPlay
  (bind _indexplayer (Variables|Default|GetIndexPlayer))
  (bind _returnvalue (Game|GetPlayerController _indexplayer))
  (bind _returnvalue_2 (PlayerController|LocalPlayerSubsystems|GetEnhancedInputLocalPlayerSubsystem _returnvalue))
  (Development|PrintString (Utilities|String|ToString(Integer) _indexplayer))
  ;[1 1 1] Set IMC
  (Utilities|IsValid _returnvalue_2
    (:Is%20Valid
      (Input|AddMappingContext _returnvalue_2 (Variables|Refs|GetMappingContext) 0 "(bIgnoreAllPressedKeysUntilRelease=True,bForceImmediately=False)"))))

(fn ConstructionScript)